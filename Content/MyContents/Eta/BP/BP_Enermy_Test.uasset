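; Test enemy Blueprint with a walk-speed setter and a Box trigger that detects BP_CheckCharacter.
; Box begin and end overlap events cast the other actor to BP_CheckCharacter and toggle the IsOverrap flag, which nothing in this graph reads.
; The Speed function sets CharacterMovement's MaxWalkSpeed from its input.
; BeginPlay and Tick only call the parent, and BeginOverrap is an empty stub.
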(event `self.ReceiveBeginPlay`
  (`parent.ReceiveBeginPlay`))

(event `self.ReceiveTick`
  (params (DeltaSeconds :type "Float (single-precision)"))
  (`parent.ReceiveTick` DeltaSeconds))

(event `self.Box.OnComponentBeginOverlap`
  (params (OverlappedComponent :type "PrimitiveComponent Object Reference") (OtherActor :type "Actor Object Reference") (OtherComp :type "PrimitiveComponent Object Reference") (OtherBodyIndex :type Integer) (bFromSweep :type Boolean) (SweepResult :type "HitResult Structure (by ref)"))
  (cast `/Game/MyContents/Eta/BP_CheckCharacter` OtherActor)
  (set `self.bIsOverrap` true))

(event `self.Box.OnComponentEndOverlap`
  (params (OverlappedComponent :type "PrimitiveComponent Object Reference") (OtherActor :type "Actor Object Reference") (OtherComp :type "PrimitiveComponent Object Reference") (OtherBodyIndex :type Integer))
  (cast `/Game/MyContents/Eta/BP_CheckCharacter` OtherActor)
  (set `self.bIsOverrap` false))

(fn `BeginOverrap`)

(fn `Speed`
  (params (`Max Walk Speed` :type "Float (single-precision)"))
  (set `CharacterMovementComponent.MaxWalkSpeed` `Max Walk Speed` (`self.CharacterMovement`)))

(fn `UserConstructionScript`)