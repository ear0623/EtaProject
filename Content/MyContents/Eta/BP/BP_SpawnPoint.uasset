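; Spawn point actor that creates a batch of enemies around itself when play begins.
; It finds an existing BP_Enermy in the level and fills the AddSlot array with repeated references to it.
; A loop spawns that enemy's class at random picks from five fixed diagonal offsets around the actor.
; Each spawn removes its slot during iteration, so the loop skips entries and spawns fewer enemies than queued.
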(event `self.ReceiveBeginPlay`
  (bind _returnvalue (`GameplayStatics.GetActorOfClass` "/Game/MyContents/Eta/BP/BP_Enermy.BP_Enermy_C"))
  (bind _output_get (set `self.BP_Enermy` _returnvalue))
  (`self.InitEnermy` _output_get)
  (`self.SpawnEnermy`))

(event `InitEnermy`
  (params (Enermy :type "Actor Object Reference (by ref)"))
  (for _ (range 6)
    (`KismetArrayLibrary.Array_Add` (`self.AddSlot`) Enermy)))

(event `SpawnEnermy`
  (bind _returnvalue_location (`KismetMathLibrary.BreakTransform` (`self.GetTransform` self)))
  (for (_array_element _array_index) (`self.AddSlot`)
    (if (== _array_element (`self.BP_Enermy`))
      (`|SpawnActorFromClass` (`GameplayStatics.GetObjectClass` (`self.BP_Enermy`)) (`KismetMathLibrary.MakeTransform` (`KismetArrayLibrary.Array_Random` (`|MakeArray` _returnvalue_location (+ _returnvalue_location (100.0 100.0 0.0)) (+ _returnvalue_location (-100.0 -100.0 0.0)) (+ _returnvalue_location (200.0 200.0 0.0)) (+ _returnvalue_location (-200.0 -200.0 0.0))))) "Undefined" "MultiplyWithRoot" null null)
      (`KismetArrayLibrary.Array_Remove` (`self.AddSlot`) _array_index))))

(fn `UserConstructionScript`)